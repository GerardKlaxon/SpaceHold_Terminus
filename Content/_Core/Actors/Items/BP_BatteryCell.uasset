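; BP_BatteryCell is a battery item that the player can pick up.
; Its Box overlap flags the player as able to interact and registers the cell as the interaction target, then clears both on exit.
; Interact reuses the character cast from the begin overlap, passes the cell to that character's PickUpItem and prints a green debug message.
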(event `/Game/_Core/Actors/Systems/Workshop/BPI_Interactions.Interact`
  (`/Game/_Core/Actors/Players/BP_PlayerCharacter.Pick Up Item` (stale `self.Box.OnComponentBeginOverlap` _asbp_player_character) (stale `self.Box.OnComponentBeginOverlap` _output_get) self)
  (`KismetSystemLibrary.PrintString` "YES" true true (struct :`G` 1.0 :`B` 0.112068 :`A` 1.0)))

(event `self.Box.OnComponentBeginOverlap`
  (params (OverlappedComponent :type "PrimitiveComponent Object Reference") (OtherActor :type "Actor Object Reference") (OtherComp :type "PrimitiveComponent Object Reference") (OtherBodyIndex :type Integer) (bFromSweep :type Boolean) (SweepResult :type "HitResult Structure (by ref)"))
  (bind _asbp_player_character (cast `/Game/_Core/Actors/Players/BP_PlayerCharacter` OtherActor))
  (set `/Game/_Core/Actors/Players/BP_PlayerCharacter.canInteract` true _asbp_player_character)
  (bind _output_get (set `/Game/_Core/Actors/Players/BP_PlayerCharacter.InteractionActorREF` self _asbp_player_character)))

(event `self.Box.OnComponentEndOverlap`
  (params (OverlappedComponent :type "PrimitiveComponent Object Reference") (OtherActor :type "Actor Object Reference") (OtherComp :type "PrimitiveComponent Object Reference") (OtherBodyIndex :type Integer))
  (bind _asbp_player_character (cast `/Game/_Core/Actors/Players/BP_PlayerCharacter` OtherActor))
  (set `/Game/_Core/Actors/Players/BP_PlayerCharacter.canInteract` false _asbp_player_character)
  (set `/Game/_Core/Actors/Players/BP_PlayerCharacter.InteractionActorREF` null _asbp_player_character))

(fn `UserConstructionScript`)