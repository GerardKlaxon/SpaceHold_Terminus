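; Parent ore actor that a player drills to collect ore into their inventory.
; A box overlap registers one player at a time and shares a FlipFlop between enter and exit to toggle that player's drill ability.
; Drilling calls raise progress on a widget bar until toughness is reached, then the ore goes to the PlayerState and the actor is destroyed.
; Leaving resets progress; the GameState global score call is disconnected.
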(event `self.ReceiveBeginPlay`
  (bind _asbpw_drill_progress_bar (cast `/Game/_Core/UI/BPW_DrillProgressBar` (`WidgetComponent.GetWidget` (`self.Widget`))))
  (set `self.As BPW Drill Progress Bar` _asbpw_drill_progress_bar))

(event `self.Box.OnComponentBeginOverlap`
  (params (OverlappedComponent :type "PrimitiveComponent Object Reference") (OtherActor :type "Actor Object Reference") (OtherComp :type "PrimitiveComponent Object Reference") (OtherBodyIndex :type Integer) (bFromSweep :type Boolean) (SweepResult :type "HitResult Structure (by ref)"))
  (bind _as_bp_player_character (`self.As BP Player Character`))
  (if (`self.noPlayer`)
    (bind _asbp_player_character (cast `/Game/_Core/Actors/Players/BP_PlayerCharacter` OtherActor))
    (set `self.As BP Player Character` _asbp_player_character)
    (set `self.noPlayer` false)
    (`/Engine/EditorBlueprintResources/StandardMacros.FlipFlop` :!label _label
      (:`A`
        (`/Game/_Core/Actors/Players/BP_PlayerCharacter.Drill` _as_bp_player_character true self))
      (:`B`
        (`/Game/_Core/Actors/Players/BP_PlayerCharacter.Drill` _as_bp_player_character false self)))))

(event `self.Box.OnComponentEndOverlap`
  (params (OverlappedComponent :type "PrimitiveComponent Object Reference") (OtherActor :type "Actor Object Reference") (OtherComp :type "PrimitiveComponent Object Reference") (OtherBodyIndex :type Integer))
  (if (`self.noPlayer`)
    _
    (elif (== OtherActor (`self.As BP Player Character`))
      (bind _output_get (set `self.Drill Progress` 0.0))
      (`/Game/_Core/UI/BPW_DrillProgressBar.UpdateDrillProgress` (`self.As BPW Drill Progress Bar`) _output_get)
      (set `self.noPlayer` true)
      (goto _label))))

(event `ResetDrillProgress`
  (bind _output_get (set `self.Drill Progress` 0.0))
  (`/Game/_Core/UI/BPW_DrillProgressBar.UpdateDrillProgress` (`self.As BPW Drill Progress Bar`) _output_get))

(event `Drilling`
  (bind _drill_progress (`self.Drill Progress`))
  (if (< _drill_progress (`self.DrillToughness`))
    (bind _result (`/Engine/EditorBlueprintResources/StandardMacros.IncrementFloat` _drill_progress)
      (:`  `
        (`KismetSystemLibrary.PrintString` (`KismetStringLibrary.Conv_DoubleToString` _result) true true (struct :`R` 0.177083 :`G` 0.039221 :`B` 0.025107 :`A` 1.0) 0.0)
        (`/Game/_Core/UI/BPW_DrillProgressBar.UpdateDrillProgress` (`self.As BPW Drill Progress Bar`) _result)))
    (else
      (`self.Drilled`))))

(event `Drilled`
  (bind _asps_player_character (cast `/Game/_Core/Actors/Players/PS_PlayerCharacter` (`Pawn.PlayerState` (`self.As BP Player Character`))))
  (`/Game/_Core/Actors/Players/PS_PlayerCharacter.AddOreToInventory` _asps_player_character (`self.OreType`) (`self.OreAmount`))
  (`self.K2_DestroyActor`))

(fn `UserConstructionScript`)