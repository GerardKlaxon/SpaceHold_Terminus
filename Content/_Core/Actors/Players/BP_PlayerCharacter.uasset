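; Networked player character that moves, aims and drills ore through Enhanced Input.
; Movement and, for one controller type, look input turn a placeholder Cube locally, then relay yaw through server-to-multicast events.
; Drill stores the current ore and permission, letting input drive server events that advance or reset that ore's progress.
; A debug input asks GS_BaseGame to retrieve global resources; drill UI is unfinished.
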(event Custom|Drill
  (params (canDrill :type Boolean) (OreREF :type BP%20Ore%20Parent%20Object%20Reference))
  (Variables|Drill|SetcanDrill canDrill)
  (bind _output_get (Variables|Ore|SetOreREF OreREF)))

(event Custom|SERVER_CharaLookRot
  (params (New%20Rotation%20Z%20%28Yaw%29 :type Float%20%28single-precision%29))
  ;[0.02604 0.02604 0.02604] Movement And Character Direction
  (CallFunction|MULTICharaLookRot New%20Rotation%20Z%20%28Yaw%29))

(event Custom|MULTI_CharaLookRot
  (params (New%20Rotation%20Z%20%28Yaw%29 :type Float%20%28single-precision%29))
  ;[0.02604 0.02604 0.02604] Movement And Character Direction
  ;;[0 0.801 1] TEMP
  ;; (Change to Mesh rotation)
  (Transformation|SetWorldRotation (Variables|Default|GetCube) (Math|Rotator|MakeRotator 0.0 0.0 New%20Rotation%20Z%20%28Yaw%29) false false))

(event Custom|SERVER_CharaRot
  (params (New%20Rotation%20Z%20%28Yaw%29 :type Float%20%28single-precision%29))
  ;[0.02604 0.02604 0.02604] Movement And Character Direction
  (CallFunction|MULTICharaRot New%20Rotation%20Z%20%28Yaw%29))

(event Custom|MULTI_CharaRot
  (params (New%20Rotation%20Z%20%28Yaw%29 :type Float%20%28single-precision%29))
  (bind _cube (Variables|Default|GetCube))
  (bind _returnvalue (Transformation|GetWorldRotation _cube))
  ;[0.02604 0.02604 0.02604] Movement And Character Direction
  ;;[0 0.801 1] TEMP
  ;; (Change to Mesh rotation)
  (Transformation|SetWorldRotation _cube (Math|Rotator|MakeRotator (.roll _returnvalue) (.pitch _returnvalue) New%20Rotation%20Z%20%28Yaw%29) false false))

(event Custom|AllowToMov
  ;[0.02604 0.02604 0.02604] Movement And Character Direction
  (Variables|Default|SetcanMove true))

(event Custom|SERVER_Drilling
  (Default|Drilling (stale Custom|Drill _output_get)))

(event Custom|SERVER_AccessGlobalInv
  ;[0.02604 0.02604 0.02604] Movement And Character Direction
  (bind _asgs_base_game (Utilities|Casting|CastToGS_BaseGame (Game|GetGameState)))
  (Default|SERVERRetrieveResources _asgs_base_game))

(event Custom|SERVER_ResetDrillTimer
  (Variables|/Game/_Core/Actors/Ores/BP_Ore_Parent.BP_Ore_Parent_C|SetDrill%20Progress (stale Custom|Drill _output_get) 0.0))

(event Input|EnhancedActionEvents|EnhancedInputActionIA_Action
  (params (ActionValue :type Boolean) (ElapsedSeconds :type Float%20%28double-precision%29) (TriggeredSeconds :type Float%20%28double-precision%29) (InputAction :type Input%20Action%20Object%20Reference :default "/Game/_Core/Inputs/IA_Action.IA_Action")))

(event Input|EnhancedActionEvents|EnhancedInputActionIA_Movement
  (params (ActionValue :type Vector%202D%20Structure) (ElapsedSeconds :type Float%20%28double-precision%29) (TriggeredSeconds :type Float%20%28double-precision%29) (InputAction :type Input%20Action%20Object%20Reference :default "/Game/_Core/Inputs/IA_Movement.IA_Movement"))
  (bind _returnvalue (Pawn|GetControlRotation :!class /Script/Engine.Pawn))
  (bind _returnvalue_2 (Transformation|GetActorLocation))
  (bind _returnvalue_3 (Class|KismetMathLibrary|VectorNormal2D (Math|Vector|MakeVector (.y ActionValue) (.x ActionValue) 0.0) 0.0001))
  (bind _returnvalue_4 (* _returnvalue_3 1e+01))
  (bind _returnvalue_5 (+ _returnvalue_2 _returnvalue_4))
  (bind _returnvalue_6 (Math|Rotator|FindLookatRotation _returnvalue_2 _returnvalue_5))
  ;[0.02604 0.02604 0.02604] Movement And Character Direction
  (:Triggered
    (if (Variables|Default|GetcanMove)
      (Pawn|Input|AddMovementInput (Math|Vector|GetRightVector (Math|Rotator|MakeRotator (.roll _returnvalue) 0.0 (.yaw _returnvalue))) (.x ActionValue) false)
      (Pawn|Input|AddMovementInput (Math|Vector|GetForwardVector (Math|Rotator|MakeRotator 0.0 0.0 (.yaw (Pawn|GetControlRotation :!class /Script/Engine.Pawn)))) (.y ActionValue) false)
      ;;[0 0.801 1] TEMP
      ;; (Change to Mesh rotation)
      (Transformation|SetWorldRotation (Variables|Default|GetCube) (Math|Rotator|MakeRotator (.roll _returnvalue_6) (.pitch _returnvalue_6) (.yaw _returnvalue_6)) false false)
      (CallFunction|SERVERCharaRot (.yaw _returnvalue_6)))))

(event Input|EnhancedActionEvents|EnhancedInputActionIA_DebugPlayerInv
  (params (ActionValue :type Boolean) (ElapsedSeconds :type Float%20%28double-precision%29) (TriggeredSeconds :type Float%20%28double-precision%29) (InputAction :type Input%20Action%20Object%20Reference :default "/Game/_Core/Inputs/IA_DebugPlayerInv.IA_DebugPlayerInv"))
  ;[0.02604 0.02604 0.02604] Movement And Character Direction
)

(event Input|EnhancedActionEvents|EnhancedInputActionIA_DrillModeAction
  (params (ActionValue :type Boolean) (ElapsedSeconds :type Float%20%28double-precision%29) (TriggeredSeconds :type Float%20%28double-precision%29) (InputAction :type Input%20Action%20Object%20Reference :default "/Game/_Core/Inputs/IA_DrillModeAction.IA_DrillModeAction"))
  (:Triggered
    (if (and ActionValue (Variables|Drill|GetcanDrill))
      (CallFunction|SERVERDrilling)))
  (:Completed
    (if (Class|KismetMathLibrary|XORBoolean ActionValue (Variables|Drill|GetcanDrill))
      (CallFunction|SERVERResetDrillTimer))))

(event Input|EnhancedActionEvents|EnhancedInputActionIA_Look
  (params (ActionValue :type Vector%202D%20Structure) (ElapsedSeconds :type Float%20%28double-precision%29) (TriggeredSeconds :type Float%20%28double-precision%29) (InputAction :type Input%20Action%20Object%20Reference :default "/Game/_Core/Inputs/IA_Look.IA_Look"))
  (bind _returnvalue (Transformation|GetActorLocation))
  (bind _returnvalue_2 (* (.x ActionValue) -1.0))
  (bind _returnvalue_3 (Class|KismetMathLibrary|VectorNormal2D (Math|Vector|MakeVector _returnvalue_2 (.y ActionValue) 0.0) 0.0001))
  (bind _returnvalue_4 (* _returnvalue_3 1e+01))
  (bind _returnvalue_5 (+ _returnvalue _returnvalue_4))
  (bind _returnvalue_6 (Math|Rotator|FindLookatRotation _returnvalue _returnvalue_5))
  ;[0.02604 0.02604 0.02604] Movement And Character Direction
  (:Triggered
    (if (== (Variables|Default|GetControllerType) 1)
      ;;[0 0.801 1] TEMP
      ;; (Change to Mesh rotation)
      (Transformation|SetWorldRotation (Variables|Default|GetCube) (Math|Rotator|MakeRotator (.roll _returnvalue_6) (.pitch _returnvalue_6) (.yaw _returnvalue_6)) false false)
      (CallFunction|SERVERCharaLookRot (.yaw _returnvalue_6)))))

(event Input|EnhancedActionEvents|EnhancedInputActionIA_DebugGlobalInv
  (params (ActionValue :type Boolean) (ElapsedSeconds :type Float%20%28double-precision%29) (TriggeredSeconds :type Float%20%28double-precision%29) (InputAction :type Input%20Action%20Object%20Reference :default "/Game/_Core/Inputs/IA_DebugGlobalInv.IA_DebugGlobalInv"))
  ;[0.02604 0.02604 0.02604] Movement And Character Direction
  (:Triggered
    (CallFunction|SERVERAccessGlobalInv)))

(event Input|GamepadEvents|DebugKeyGamepadFaceButtonBottom
  (params (Key :type Key%20Structure :default "None") (ActionValue :type Input%20Action%20Value%20Structure))
  ;[0 0.9826 1] TEMP
)

(fn ConstructionScript)

(fn NewFunction)