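; BP_Workshop is an interactable workshop actor that opens a workshop UI and stores an additional crafted battery.
; Box overlap marks the player character as able to interact and registers the workshop as its interaction target.
; Interact creates the BPW_WorkshopMain widget for the local controller, and leaving the box clears the interact flag and removes the widget.
; StoreObject saves the passed object and prints a debug message.
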(event `self.Box.OnComponentBeginOverlap`
  (params (OverlappedComponent :type "PrimitiveComponent Object Reference") (OtherActor :type "Actor Object Reference") (OtherComp :type "PrimitiveComponent Object Reference") (OtherBodyIndex :type Integer) (bFromSweep :type Boolean) (SweepResult :type "HitResult Structure (by ref)"))
  (bind _asbp_player_character (cast `/Game/_Core/Actors/Players/BP_PlayerCharacter` OtherActor))
  (set `/Game/_Core/Actors/Players/BP_PlayerCharacter.canInteract` true _asbp_player_character)
  (set `/Game/_Core/Actors/Players/BP_PlayerCharacter.InteractionActorREF` self _asbp_player_character))

(event `/Game/_Core/Actors/Systems/Workshop/BPI_Interactions.Interact`
  (bind _asbp_player_controller (cast `/Game/_Core/Actors/Players/BP_PlayerController` (`Pawn.GetController` (stale `self.Box.OnComponentBeginOverlap` _asbp_player_character))))
  (if (`Controller.IsLocalController` _asbp_player_controller)
    (bind _returnvalue (`|CreateWidget` "/Game/_Core/UI/WorkshopUI/BPW_WorkshopMain.BPW_WorkshopMain_C" _asbp_player_controller))
    (`UserWidget.AddToViewport` _returnvalue 0)))

(event `self.Box.OnComponentEndOverlap`
  (params (OverlappedComponent :type "PrimitiveComponent Object Reference") (OtherActor :type "Actor Object Reference") (OtherComp :type "PrimitiveComponent Object Reference") (OtherBodyIndex :type Integer))
  (bind _asbp_player_character (cast `/Game/_Core/Actors/Players/BP_PlayerCharacter` OtherActor))
  (set `/Game/_Core/Actors/Players/BP_PlayerCharacter.canInteract` false _asbp_player_character)
  (bind _asbp_player_controller (cast `/Game/_Core/Actors/Players/BP_PlayerController` (`Pawn.GetController` _asbp_player_character)))
  (if (`Controller.IsLocalController` _asbp_player_controller)
    (`GameViewportSubsystem.RemoveWidget` (subsystem `GameViewportSubsystem`) (stale `/Game/_Core/Actors/Systems/Workshop/BPI_Interactions.Interact` _returnvalue))))

(event `/Game/_Core/Actors/Systems/Workshop/BPI_Interactions.StoreObject`
  (params (`Object Stored` :type "/Game/_Core/Actors/Systems/Workshop/E_RecipeName Enum" :default "NewEnumerator3"))
  ;[0.9911 0.5271 1] Storing additional battery crafted (player can only holds one at given time)
  (set `self.Object Stored` `Object Stored`)
  (`KismetSystemLibrary.PrintString` "STOCKED" true true (struct :`R` 0.976841 :`B` 1.0 :`A` 1.0)))

(fn `UserConstructionScript`)