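; Base game mode that spawns player characters and releases their movement when play begins.
; GM_SpawnPawns destroys any pawn the controller holds, spawns a BP_PlayerCharacter at a randomly chosen PlayerStart, possesses it, then calls MULTIAddMappingContext on the controller.
; GM_PcValidity calls AllowToMov on every BP_PlayerCharacter in the level and prints a play message.
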(event `self.ReceiveBeginPlay`)

(event `GM_SpawnPawns`
  (params (`Player Controller` :type "/Game/_Core/Actors/Players/BP_PlayerController Object Reference"))
  (bind _player_controller_out (`self.SpawnPlayer` `Player Controller`))
  (`/Game/_Core/Actors/Players/BP_PlayerController.MULTI_AddMappingContext` _player_controller_out))

(event `GM_PcValidity`
  (bind _outactors (`GameplayStatics.GetAllActorsOfClass` "/Game/_Core/Actors/Players/BP_PlayerCharacter.BP_PlayerCharacter_C"))
  (for _array_element _outactors
    (`/Game/_Core/Actors/Players/BP_PlayerCharacter.AllowToMov` _array_element)
    (`KismetSystemLibrary.PrintString` "PLAY !" true true (struct :`R` 0.114405 :`G` 1.0 :`A` 1.0) 5.0)))

(fn `LocatePlayerStart`
  (returns (StartTransform :type "Transform Structure (by ref)"))
  (bind _outactors (`GameplayStatics.GetAllActorsOfClass` "/Script/Engine.PlayerStart"))
  (return (`self.GetTransform` (`|GetArrayItem` _outactors (`KismetMathLibrary.RandomIntegerInRange` 0 (- (`KismetArrayLibrary.Array_Length` _outactors) 1))))))

(fn `SpawnPlayer`
  (params (`Player Controller In` :type "/Game/_Core/Actors/Players/BP_PlayerController Object Reference"))
  (returns (`Player Controller Out` :type "/Game/_Core/Actors/Players/BP_PlayerController Object Reference"))
  (bind _returnvalue (`Controller.K2_GetPawn` `Player Controller In`))
  (`/Engine/EditorBlueprintResources/StandardMacros.IsValid` _returnvalue ; Check if Pawn is Destroyed\nto spawn another one
    (:`Is Valid`
      (`self.K2_DestroyActor` _returnvalue))
    (:`Is Not Valid`
      _))
  (bind _returnvalue_2 (`|SpawnActorFromClass` "/Game/_Core/Actors/Players/BP_PlayerCharacter.BP_PlayerCharacter_C" (`self.LocatePlayerStart`) "Undefined" "MultiplyWithRoot" null null))
  (`Controller.Possess` `Player Controller In` _returnvalue_2)
  (return `Player Controller In`))

(fn `UserConstructionScript`)